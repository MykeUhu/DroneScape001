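; BP_UhuDrone is a drone character Blueprint that runs a scripted state and task sequence on BeginPlay, apparently as a test.
; It enters emergency return mode, executes its highest-priority task, then uses delays to switch to idle and back to emergency return.
; Executed task names are written to the log; overlap and tick events are empty, and two debug prints are unconnected.
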(event EventBeginPlay
  (bind _output_get (Variables|Default|SetDrone self))
  (Class|UhuDroneCharacter|SetDroneState _output_get false false false false true)
  (Class|UhuDroneCharacter|ExecuteHighestPriorityTask)
  (Development|PrintString "Task Set")
  (Utilities|FlowControl|Delay 5.0)
  (Class|UhuDroneCharacter|SetDroneState true false false false false)
  (Utilities|FlowControl|Delay 1e+01)
  (Class|UhuDroneCharacter|SetDroneState false false false false true))

(event Collision|EventActorBeginOverlap
  (params (OtherActor :type Actor%20Object%20Reference)))

(event EventTick
  (params (DeltaSeconds :type Float%20%28single-precision%29)))

(event EventOnTaskExecuted
  (params (TaskName :type String))
  (Utilities|String|LogString TaskName))

(fn ConstructionScript)